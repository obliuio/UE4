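; BP_Ice_Actor is a temporary ice piece, filed under ReactiveWater, that widens over time and then removes itself.
; BeginPlay starts a one-shot timer of DelayTimer length that destroys the actor, and sets the current scale to MinScale.
; Tick grows the scale at a steady rate until it reaches MaxScale, applying it to the root's X and Y while Z stays fixed.
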(event `self.ReceiveBeginPlay`
  (`KismetSystemLibrary.K2_SetTimerDelegate` (delegate `DestoryEvent`) (`self.DelayTimer`))
  (set `self.CurrentScale` (`self.MinScale`)))

(event `DestoryEvent`
  (`self.K2_DestroyActor`))

(event `self.ReceiveTick`
  (params (DeltaSeconds :type "Float (single-precision)"))
  (bind _currentscale (`self.CurrentScale`))
  (if (not (>= _currentscale (`self.MaxScale`)))
    (bind _output_get (set `self.CurrentScale` (+ _currentscale (* DeltaSeconds 0.1))))
    (`SceneComponent.SetWorldScale3D` (`self.DefaultSceneRoot`) (`KismetMathLibrary.MakeVector` _output_get _output_get 1.0))))

(fn `UserConstructionScript`)